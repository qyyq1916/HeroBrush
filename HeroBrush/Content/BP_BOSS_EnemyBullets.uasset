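; BP_BOSS_EnemyBullets is a boss bullet actor that bursts on contact with anything other than its instigator.
; Both hit and overlap events on CollisionComp run the same logic: spawn the P_ky_laser02 emitter at the bullet's location and rotation, then destroy the actor.
; The graph applies no damage, and the construction script is empty.
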(event `self.CollisionComp.OnComponentHit`
  (params (HitComponent :type "PrimitiveComponent Object Reference") (OtherActor :type "Actor Object Reference") (OtherComp :type "PrimitiveComponent Object Reference") (NormalImpulse :type "Vector Structure") (Hit :type "HitResult Structure (by ref)"))
  (if (!= OtherActor (`self.GetInstigator`))
    (`GameplayStatics.SpawnEmitterAtLocation` "/Game/BeamAndLaserFX01/Particles/P_ky_laser02.P_ky_laser02" (`self.K2_GetActorLocation`) (`self.K2_GetActorRotation`))
    (`self.K2_DestroyActor`)))

(event `self.CollisionComp.OnComponentBeginOverlap`
  (params (OverlappedComponent :type "PrimitiveComponent Object Reference") (OtherActor :type "Actor Object Reference") (OtherComp :type "PrimitiveComponent Object Reference") (OtherBodyIndex :type Integer) (bFromSweep :type Boolean) (SweepResult :type "HitResult Structure (by ref)"))
  (if (!= OtherActor (`self.GetInstigator`))
    (`GameplayStatics.SpawnEmitterAtLocation` "/Game/BeamAndLaserFX01/Particles/P_ky_laser02.P_ky_laser02" (`self.K2_GetActorLocation`) (`self.K2_GetActorRotation`))
    (`self.K2_DestroyActor`)))

(fn `UserConstructionScript`)