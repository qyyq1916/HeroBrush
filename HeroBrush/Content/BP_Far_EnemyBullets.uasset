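; BP_Far_EnemyBullets is an enemy bullet, named for far enemies, that damages the player on contact.
; When its collision component overlaps a Player-tagged HeroCharacter, it passes BulletDamage to ChangeHealth as an immediate change, spawns an explosion and destroys itself.
; A blocking hit on an Enemy-tagged actor produces the same explosion and destruction without changing health.
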(event `self.CollisionComp.OnComponentHit`
  (params (HitComponent :type "PrimitiveComponent Object Reference") (OtherActor :type "Actor Object Reference") (OtherComp :type "PrimitiveComponent Object Reference") (NormalImpulse :type "Vector Structure") (Hit :type "HitResult Structure (by ref)"))
  (if (`self.ActorHasTag` OtherActor "Enemy")
    (`GameplayStatics.SpawnEmitterAtLocation` "/Game/StarterContent/Particles/P_Explosion.P_Explosion" (`self.K2_GetActorLocation`) (`self.K2_GetActorRotation`))
    (`self.K2_DestroyActor`)))

(event `self.CollisionComp.OnComponentBeginOverlap`
  (params (OverlappedComponent :type "PrimitiveComponent Object Reference") (OtherActor :type "Actor Object Reference") (OtherComp :type "PrimitiveComponent Object Reference") (OtherBodyIndex :type Integer) (bFromSweep :type Boolean) (SweepResult :type "HitResult Structure (by ref)"))
  (if (`self.ActorHasTag` OtherActor "Player")
    (bind _ashero_character (cast `HeroCharacter` OtherActor))
    (`HeroCharacter.ChangeHealth` _ashero_character false 0 (`self.BulletDamage`))
    (`GameplayStatics.SpawnEmitterAtLocation` "/Game/StarterContent/Particles/P_Explosion.P_Explosion" (`self.K2_GetActorLocation`) (`self.K2_GetActorRotation`))
    (`self.K2_DestroyActor`)))

(fn `UserConstructionScript`)